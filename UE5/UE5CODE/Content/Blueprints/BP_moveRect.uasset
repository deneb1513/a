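; BP_moveRect is a Blueprint that moves its StaticMesh1 component along a rectangular path in the local X-Z plane, looping continuously.
; Tick switches on the Movetype state (Right, Up, Left, Down), stepping the stored X or Z position and applying it as relative location.
; Each state hands over to the next at a hard-coded bound.
; Steps are fixed per frame, so speed depends on frame rate.
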(event `self.ReceiveTick`
  (params (DeltaSeconds :type "Float (single-precision)"))
  (switch `/Game/Blueprints/EN_movetype` (`self.movetype`)
    (:`NewEnumerator0`
      ;[1 1 1] 오른쪽으로 이동
      (bind _output_get (set `self.x위치` (+ (`self.x위치`) 1.0)))
      (`SceneComponent.K2_SetRelativeLocation` (`self.StaticMesh1`) (`KismetMathLibrary.MakeVector` _output_get 0.0 (`self.Z위치`)) false false)
      ;;[1 1 1] if문. 조건을 만족하면 True로 진행
      (if (>= (`self.x위치`) 200.0)
        ;[1 1 1] 이동 타입을 바꿔주는 부분
        (set `self.movetype` "NewEnumerator1")))
    (:`NewEnumerator1`
      ;[1 1 1] 위로이동
      (bind _output_get_2 (set `self.Z위치` (+ (`self.Z위치`) 1.0)))
      (`SceneComponent.K2_SetRelativeLocation` (`self.StaticMesh1`) (`KismetMathLibrary.MakeVector` (`self.x위치`) 0.0 _output_get_2) false false)
      (if (>= (`self.Z위치`) 200.0)
        (set `self.movetype` "NewEnumerator2")))
    (:`NewEnumerator2`
      ;[1 1 1] 왼쪽으로 이동
      (bind _output_get_3 (set `self.x위치` (+ (`self.x위치`) -1.0)))
      (`SceneComponent.K2_SetRelativeLocation` (`self.StaticMesh1`) (`KismetMathLibrary.MakeVector` _output_get_3 0.0 (`self.Z위치`)) false false)
      (if (<= (`self.x위치`) -200.0)
        (set `self.movetype` "NewEnumerator3")))
    (:`NewEnumerator3`
      ;[1 1 1] 아래로 이동
      (bind _output_get_4 (set `self.Z위치` (+ (`self.Z위치`) -1.0)))
      (`SceneComponent.K2_SetRelativeLocation` (`self.StaticMesh1`) (`KismetMathLibrary.MakeVector` (`self.x위치`) 0.0 _output_get_4) false false)
      (if (<= (`self.Z위치`) -200.0)
        (set `self.movetype` "NewEnumerator0")))))

(fn `UserConstructionScript`)