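; BP_moveleftright is an actor whose mesh slides back and forth along relative X between fixed limits while Isplay is true.
; Tick moves it a fixed step per frame, independent of delta time, flipping direction at each limit.
; BeginPlay binds to the referenced BPSwitch's overlap dispatcher, or prints a warning if that reference is unset.
; EventOverlap and DoPlay both set Isplay to start or pause the motion.
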(event `self.ReceiveBeginPlay`
  (bind _bp_switch (`self.BP_Switch`))
  ;[1 1 1] 정상작동 확인
  (`/Engine/EditorBlueprintResources/StandardMacros.IsValid` _bp_switch
    (:`Is Valid`
      ;[1 1 1] 이벤트에 바인딩(연결)한다.
      (add `/Game/Blueprints/BP_Switch.NewEventDispatcher_OverLab` _bp_switch (`|CreateDelegate` :!event `Event_Overlap`)))
    (:`Is Not Valid`
      (`KismetSystemLibrary.PrintString` (`KismetStringLibrary.Concat_StrStr` (`KismetSystemLibrary.GetDisplayName` self) "에 디테일에 스위치 객체 정보를 안넣었음") true true (struct :`G` 0.66 :`B` 1.0 :`A` 1.0) 5.0))))

(event `self.ReceiveTick`
  (params (DeltaSeconds :type "Float (single-precision)"))
  (if (`self.Isplay`)
    (if (`self.오른쪽방향 진행`)
      ;[1 1 1] 오른쪽으로 이동
      (bind _output_get (set `self.x위치` (+ (`self.x위치`) 1.0)))
      (`SceneComponent.K2_SetRelativeLocation` (`self.StaticMesh1`) (`KismetMathLibrary.MakeVector` _output_get) false false)
      (if (>= (`self.x위치`) 200.0)
        (set `self.오른쪽방향 진행` false))
      (else
        ;[1 1 1] 왼쪽으로 이동
        (bind _output_get_2 (set `self.x위치` (+ (`self.x위치`) -1.0)))
        (`SceneComponent.K2_SetRelativeLocation` (`self.StaticMesh1`) (`KismetMathLibrary.MakeVector` _output_get_2) false false)
        (if (<= (`self.x위치`) -200.0)
          (set `self.오른쪽방향 진행` true))))))

(fn `DoPlay`
  (params (Isplay :type Boolean))
  (returns (BResult :type Boolean))
  (set `self.Isplay` Isplay)
  (return false))

(fn `Event_Overlap`
  (params (IsBegin :type Boolean))
  (set `self.Isplay` IsBegin))

(fn `UserConstructionScript`)